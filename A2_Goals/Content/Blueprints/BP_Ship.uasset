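; BP_Ship is a ship actor that turns with its movement and shows whether it is tracked.
; Each tick, a non-zero MovementDirection eases rotation via RInterpTo at RotationSpeed, with the look-at reversed so forward X points opposite the movement.
; Tick also writes IsTracked as the "Selected" material scalar on the Base, Cone and Post components.
; The graph only reads MovementDirection and IsTracked, and never moves the ship.
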(event EventBeginPlay)

(event Collision|EventActorBeginOverlap
  (params (OtherActor :type Actor%20Object%20Reference)))

(event EventTick
  (params (DeltaSeconds :type Float%20%28single-precision%29))
  (bind _returnvalue (Transformation|GetActorLocation))
  (bind _movementdirection (Variables|Default|GetMovementDirection))
  ;[1 1 1] Set Rotation
  (if (Math|Vector|VectorIsZero _movementdirection)
    _
    (else
      (Transformation|SetActorRotation (Math|Interpolation|RInterpTo (Transformation|GetActorRotation) (Math|Rotator|FindLookatRotation (+ _movementdirection _returnvalue) _returnvalue) DeltaSeconds (Variables|Default|GetRotation%20Speed)))))
  ;[1 1 1] Update the Material
  (Rendering|Material|SetScalarParameterValueonMaterials (Variables|Default|GetBase) "Selected" (Math|Conversions|ToFloat(Boolean) (Variables|Default|GetIsTracked))))

(fn ConstructionScript)